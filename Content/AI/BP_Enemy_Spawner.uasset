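; BP_Enemy_Spawner is an enemy spawner kept as old reference code, with BeginPlay and SpawnEnemy left empty.
; EnemyDeath decrements EnemyAmount and prints it through the PrintEnemyAmount debug function.
; Disconnected nodes hold the former logic: a looping timer, and a count-capped spawn of BP_AI at a random reachable point that could then move toward Tpc.
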(event `self.ReceiveBeginPlay`
  ;[1 1 1] old code keeping for reference
)

(event `SpawnEnemy`
  ;[1 1 1] old code keeping for reference
)

(event `EnemyDeath`
  ;[1 1 1] old code keeping for reference
  (`/Engine/EditorBlueprintResources/StandardMacros.DecrementInt` (`self.EnemyAmount`)
    (:`  `
      (`self.PrintEnemyAmount`))))

(fn `UserConstructionScript`)