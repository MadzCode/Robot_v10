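; Enemy AI character that wanders to random reachable points until pawn sensing spots a pawn, then continually chases the player.
; Its damage box calls the player's hit handler on overlap and applies damage to itself when touched by bullets or knives.
; Damage lowers health and updates a widget health bar; at zero it explodes, ragdolls, notifies the enemy spawner and is destroyed after a delay.
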(event `self.ReceiveBeginPlay`
  ;[1 1 1] Set current health
  (`self.FollowPlayer`)
  (bind _returnvalue (`GameplayStatics.GetActorOfClass` "/Game/AI/BP_Enemy_Spawner.BP_Enemy_Spawner_C"))
  (set `self.As BP  Enemy Spawner` _returnvalue)
  (bind _asai_health (cast `/Game/UI/AI_Health` (`WidgetComponent.GetUserWidgetObject` (`self.HealthWidget`))))
  (bind _output_get (set `self.AI Health` _asai_health))
  (set `/Game/UI/AI_Health.CurrentHealth` (`self.CurrentHealth`) _output_get)
  (set `/Game/UI/AI_Health.MaxHealth` (`self.MaxHealth`) _output_get))

(event `self.PawnSensing.OnSeePawn`
  (params (Pawn :type "Pawn Object Reference"))
  ;[1 1 1] Follow Player
  (set `self.SeesPlayer?` true)
  (`self.FollowPlayer`))

(event `FollowPlayer`
  ;[1 1 1] Follow Player
  (if (`self.SeesPlayer?`)
    (`|AIMoveTo` self (0.0 0.0 0.0) (`GameplayStatics.GetPlayerCharacter` 0)
      (:`OnSuccess`
        (`self.FollowPlayer`)))
    (else
      (`|AIMoveTo` self (`NavigationSystemV1.K2_GetRandomReachablePointInRadius` (`self.K2_GetActorLocation`) 3000.0 null null) null
        (:`OnSuccess`
          (`KismetSystemLibrary.Delay` 3.0)
          (`self.FollowPlayer`))))))

(event `self.Damage_Box.OnComponentBeginOverlap`
  (params (OverlappedComponent :type "PrimitiveComponent Object Reference") (OtherActor :type "Actor Object Reference") (OtherComp :type "PrimitiveComponent Object Reference") (OtherBodyIndex :type Integer) (bFromSweep :type Boolean) (SweepResult :type "HitResult Structure (by ref)"))
  (`|ExecutionSequence`
    (:`then_0`
      ;[1 1 1] Apply Damage to player
      (bind _asbp_third_person_character (cast `/Game/ThirdPerson/Blueprints/BP_ThirdPersonCharacter` OtherActor))
      (`/Game/ThirdPerson/Blueprints/BP_ThirdPersonCharacter.AI_HIt` _asbp_third_person_character))
    (:`then_1`
      ;[1 1 1] Apply Damage to AI
      (cast `/Game/Pickup_Objs/BulletBP` OtherActor)
      (`GameplayStatics.ApplyDamage` self 0.3 :!label _label))
    (:`then_2`
      (cast `/Game/Pickup_Objs/BP_Knife` OtherActor)
      (goto _label))))

(event `self.ReceiveAnyDamage`
  (params (Damage :type "Float (single-precision)") (DamageType :type "DamageType Object Reference") (InstigatedBy :type "Controller Object Reference") (DamageCauser :type "Actor Object Reference"))
  ;[1 1 1] Damage/Death
  (set `self.CurrentHealth` (- (`self.CurrentHealth`) (* Damage 100.0)))
  (`/Game/UI/AI_Health.UpdateHealth` (`self.AI Health`) 0)
  (if (<= (`self.CurrentHealth`) 0)
    (`CharacterMovementComponent.DisableMovement` (`self.CharacterMovement`))
    (`self.DisableInput` null)
    (`GameplayStatics.SpawnEmitterAttached` "/Game/StarterContent/Particles/P_Explosion.P_Explosion" (`self.Mesh`))
    (`/Game/AI/BP_Enemy_Spawner.EnemyDeath` (`self.As BP  Enemy Spawner`))
    (`PrimitiveComponent.SetSimulatePhysics` (`self.Mesh`) true)
    (`KismetSystemLibrary.Delay` 5.0)
    (`self.K2_DestroyActor`)))

(fn `UserConstructionScript`)